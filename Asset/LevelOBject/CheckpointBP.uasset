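; Checkpoint flag actor that a player activates by overlapping it once its EssentialEnemies list is empty.
; Activation swaps the flag material, attaches an aura effect to the player, plays sound and confetti, and latches Toggled; a non-empty list plays a denial sound.
; On BeginPlay it shows the activated flag if the GameInstance checkpoint reaches its PriorityCheckpoint, without setting Toggled.
; The graph neither saves progress nor updates the enemy list.
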(event EventBeginPlay
  (bind _output_get (Variables|Default|SetGameInstance (.AsMy%20Game%20Instance%20Mini%20Company (Utilities|Casting|CastToMyGameInstanceMiniCompany (Game|GetGameInstance)))))
  (if (>= (Class|MyGameInstanceMiniCompany|GetCurrentCheckpoint _output_get) (Variables|Default|GetPriorityCheckpoint))
    (Rendering|Material|SetMaterial (Variables|Default|GetFlagPlane1) 0 "/Game/Asset/Material/M_FlagLogo.M_FlagLogo")))

(event Collision|EventActorBeginOverlap
  (params (OtherActor :type Actor%20Object%20Reference))
  (if (not (Variables|Default|GetToggled))
    (bind _asplayer_bp (Utilities|Casting|CastToPlayerBP OtherActor))
    (if (== (Utilities|Array|Length (Variables|Default|GetEssentialEnemies)) 0)
      (Effects|SpawnEmitterAttached "/Game/Asset/InfinityBladeEffects/Effects/FX_Skill_Aura/P_Aura_Default_Upheaval_01.P_Aura_Default_Upheaval_01" (Variables|/Script/Engine.Character|GetCapsuleComponent _asplayer_bp) "None")
      (Rendering|Material|SetMaterial (Variables|Default|GetFlagPlane1) 0 "/Game/Asset/Material/M_FlagLogo.M_FlagLogo")
      (Audio|PlaySoundatLocation "/Game/Asset/Sounds/Checkpoint/checkpoint.checkpoint" (Transformation|GetActorLocation) "0, 0, 0" 1.0 1.0 0.0 0 0 0)
      (Components|Activation|Activate (Variables|Default|GetConfettiParticle) false)
      (Variables|Default|SetToggled true)
      (else
        (Audio|PlaySound2D "/Game/Asset/Sounds/Non.Non" (* (Variables|Default|GetCannot%20volume) (Variables|/Script/MiniCompany.MyGameInstanceMiniCompany|GetEffectVolume (Variables|Default|GetGameInstance))) 1.0 0.0 0 0)))))

(fn ConstructionScript)