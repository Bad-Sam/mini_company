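; Player Blueprint for a company of soldiers, layering feedback, menu and lobby input onto formation and dash state.
; Tick fires a particle and rumble once per dash via a resettable DoOnce and mirrors Formation into PlayerActualFormation for the trail.
; Formation inputs play sound and rumble and pulse trigger-highlight flags, while other keys open the in-game menu or leave the lobby for LevelMap.
; EnemyCompanyDefeated plays a defeat sound on each soldier.
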(event EventTick
  (params (DeltaSeconds :type Float%20%28single-precision%29))
  ;[1 1 1] Dash feedback
  (Utilities|FlowControl|Sequence
    (:then_0
      (if (Variables|Default|GetIsDashing)
        (Utilities|FlowControl|DoOnce false :!label _label
          (:Completed
            (Effects|SpawnEmitterAttached (Variables|Default|GetParticleDash_ref) (Components|GetChildComponent (Variables|Default|GetCapsuleComponent) 0) "None" "280.000000, 0, 0" "0, 0, 0" "2.000000,2.000000,0.500000")
            (Game|Feedback|PlayDynamicForceFeedback (Game|GetPlayerController 0) 0.5 0.6 true true true true)))
        (else
          (goto _label Reset))))
    (:then_1
      ;[1 1 1] Set variable for trail
      (Variables|Default|SetplayerActualFormation (Variables|Default|GetFormation)))))

(event EventBeginPlay
  (bind _asmy_game_instance_mini_company (Utilities|Casting|CastToMyGameInstanceMiniCompany (Game|GetGameInstance)))
  (Variables|Default|SetGameInstance _asmy_game_instance_mini_company))

(event Input|ActionEvents|InputActionNextFormation
  (params (Key :type Key%20Structure :default "None"))
  ;[1 1 1] Switch Formation Event
  (:Pressed
    (Variables|Default|SetRTWhiteActivate true)
    ;;[1 1 1] Sounds
    (Audio|PlaySoundatLocation "/Game/Asset/Sounds/Formation_switch.Formation_switch" (Transformation|GetActorLocation) "0, 0, 0" (Variables|/Script/MiniCompany.MyGameInstanceMiniCompany|GetEffectVolume (Variables|Default|GetGameInstance)) 1.0 0.0 "/Game/Asset/Sounds/SoundAttenuation.SoundAttenuation" 0 0)
    (Game|Feedback|PlayDynamicForceFeedback (Game|GetPlayerController 0) 0.3 0.2 true true true true)
    (Variables|Default|SetRTWhiteActivate false)
    (Variables|Default|SetLTWhiteActivate false)))

(event Input|ActionEvents|InputActionPreviousFormation
  (params (Key :type Key%20Structure :default "None"))
  ;[1 1 1] Switch Formation Event
  (:Pressed
    (Variables|Default|SetLTWhiteActivate true)
    ;;[1 1 1] Sounds
    (Audio|PlaySoundatLocation "/Game/Asset/Sounds/Formation_switch.Formation_switch" (Transformation|GetActorLocation) "0, 0, 0" (Variables|/Script/MiniCompany.MyGameInstanceMiniCompany|GetEffectVolume (Variables|Default|GetGameInstance)) 1.0 0.0 "/Game/Asset/Sounds/SoundAttenuation.SoundAttenuation" 0 0)
    (Game|Feedback|PlayDynamicForceFeedback (Game|GetPlayerController 0) 0.3 0.2 true true true true)
    (Variables|Default|SetRTWhiteActivate false)
    (Variables|Default|SetLTWhiteActivate false)))

(event Input|GamepadEvents|GamepadSpecialRight
  (params (Key :type Key%20Structure :default "None"))
  ;[1 1 1] Start Menu
  (:Pressed
    (Default|StartinGameMenu (Variables|Default|GetHUD))))

(event Input|GamepadEvents|GamepadSpecialLeft
  (params (Key :type Key%20Structure :default "None"))
  (bind _gameinstance (Variables|Default|GetGameInstance))
  ;[1 1 1] Input To quit Lobby
  (:Pressed
    (if (Variables|/Script/MiniCompany.MyGameInstanceMiniCompany|GetInLobby _gameinstance)
      (Variables|/Script/MiniCompany.MyGameInstanceMiniCompany|SetInLobby _gameinstance false)
      (Class|MyGameInstanceMiniCompany|Reset (Variables|Default|GetGameInstance) true)
      (Game|OpenLevel(byName) "LevelMap"))))

(event Input|KeyboardEvents|Escape
  (params (Key :type Key%20Structure :default "None"))
  ;[1 1 1] Start Menu
  (:Pressed
    (Default|StartinGameMenu (Variables|Default|GetHUD))))

(event Input|KeyboardEvents|P
  (params (Key :type Key%20Structure :default "None"))
  ;[1 1 1] Start Menu
  (:Pressed
    (Default|StartinGameMenu (Variables|Default|GetHUD))))

(event Input|KeyboardEvents|Enter
  (params (Key :type Key%20Structure :default "None"))
  (bind _gameinstance (Variables|Default|GetGameInstance))
  ;[1 1 1] Input To quit Lobby
  (:Pressed
    (if (Variables|/Script/MiniCompany.MyGameInstanceMiniCompany|GetInLobby _gameinstance)
      (Variables|/Script/MiniCompany.MyGameInstanceMiniCompany|SetInLobby _gameinstance false)
      (Class|MyGameInstanceMiniCompany|Reset (Variables|Default|GetGameInstance) true)
      (Game|OpenLevel(byName) "LevelMap"))))

(fn ConstructionScript)

(fn EnemyCompanyDefeated
  (for _array_element (Variables|Default|GetSoldiers)
    (Audio|SpawnSoundAttached "/Game/Asset/Sounds/Company_defeated.Company_defeated" (Variables|/Script/Engine.Character|GetCapsuleComponent _array_element) "None" "0, 0, 0" "0, 0, 0" "KeepRelativeOffset" false (* (Variables|Default|GetCompany%20defeated%20volume) (Variables|/Script/MiniCompany.MyGameInstanceMiniCompany|GetEffectVolume (Variables|Default|GetGameInstance))) 1.0 0.0 "/Game/Asset/Sounds/SoundAttenuation.SoundAttenuation" 0)))