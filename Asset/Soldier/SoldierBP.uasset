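; Soldier character Blueprint that drives its animation and plays a jump sound.
; Each Tick, it projects velocity onto the actor's forward and right vectors, divides by max movement speed, and writes the results to SoldierAnim's input values.
; On jump, it plays a sound at its location, scaled by the effect volume from the game instance cached at BeginPlay.
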(event EventOnJumped
  ;[1 1 1] Sound
  (Audio|PlaySoundatLocation "/Game/Asset/Sounds/Saut/jump.jump" (Transformation|GetActorLocation) "0, 0, 0" (* 0.1 (Variables|/Script/MiniCompany.MyGameInstanceMiniCompany|GetEffectVolume (Variables|Default|GetGameInstance))) 1.0 0.0 "/Game/Asset/Sounds/SoundAttenuation.SoundAttenuation" 0 0))

(event EventBeginPlay
  (Variables|Default|SetGameInstance (.AsMy%20Game%20Instance%20Mini%20Company (Utilities|Casting|CastToMyGameInstanceMiniCompany (Game|GetGameInstance)))))

(event EventTick
  (params (DeltaSeconds :type Float%20%28single-precision%29))
  (bind _returnvalue (Transformation|GetVelocity))
  (bind _charactermovement (Variables|Character|GetCharacterMovement))
  (bind _soldieranim (Variables|Default|GetSoldierAnim))
  (bind _returnvalue_2 (Class|MovementComponent|GetMaxSpeed _charactermovement))
  ;[1 1 1] Animation synchronizing
  (Variables|/Script/MiniCompany.SoldierAnim|SetForwardInputValue _soldieranim (Math|Float|SafeDivide (Math|Vector|DotProduct (Transformation|GetActorForwardVector) _returnvalue) _returnvalue_2))
  (Variables|/Script/MiniCompany.SoldierAnim|SetSideInputValue _soldieranim (Math|Float|SafeDivide (Math|Vector|DotProduct _returnvalue (Transformation|GetActorRightVector)) _returnvalue_2)))

(fn ConstructionScript)