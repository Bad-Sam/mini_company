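; Player soldier Blueprint that handles sword trail visuals and impact feedback.
; TrailBeginEvent picks a blue, red or green trail template from the leader's triangle, line or circle formation, with per-formation toggles so the trail only restarts on a formation change.
; TrailEndEvent ends the trail and clears the toggles.
; ImpactPlayerEvent spawns a particle at a fixed world-axis offset from the soldier and briefly vibrates the first player's controller.
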(event Custom|TrailBeginEvent
  ;[1 1 1] Colored trail
  (switch Utilities|FlowControl|Switch|SwitchonFormationType (Variables|/Script/MiniCompany.CompanyLeader|GetFormation (Class|Soldier|GetLeader))
    (:TRIANGLE
      (Variables|Default|SetLineToggle false)
      (Variables|Default|SetCircleToggle false)
      (if (not (Variables|Default|GetTriangleToggle))
        (Effects|Components|ParticleSystem|SetTemplate (Variables|Default|GetSwordTrail) "/Game/Asset/Particles/P_TrailSwordBlue.P_TrailSwordBlue")
        (Variables|Default|SetTriangleToggle true)
        (Effects|Particles|Trails|BeginTrails (Variables|Default|GetSwordTrail) "hand_rSocket" "hand_rSocket_1" "ETrailWidthMode_FromCentre" 1.0 :!label _label)))
    (:LINE
      (Variables|Default|SetTriangleToggle false)
      (Variables|Default|SetCircleToggle false)
      (if (not (Variables|Default|GetLineToggle))
        (Effects|Components|ParticleSystem|SetTemplate (Variables|Default|GetSwordTrail) "/Game/Asset/Particles/P_TrailSwordRed.P_TrailSwordRed")
        (Variables|Default|SetLineToggle true)
        (goto _label)))
    (:CIRCLE
      (Variables|Default|SetLineToggle false)
      (Variables|Default|SetTriangleToggle false)
      (if (not (Variables|Default|GetCircleToggle))
        (Effects|Components|ParticleSystem|SetTemplate (Variables|Default|GetSwordTrail) "/Game/Asset/Particles/P_TrailSwordGreen.P_TrailSwordGreen")
        (Variables|Default|SetCircleToggle true)
        (goto _label)))))

(event Custom|TrailEndEvent
  ;[1 1 1] Colored trail
  ;;[1 1 1] Reset trail
  (Effects|Particles|Trails|EndTrails (Variables|Default|GetSwordTrail))
  (Variables|Default|SetTriangleToggle false)
  (Variables|Default|SetCircleToggle false)
  (Variables|Default|SetLineToggle false))

(event Custom|ImpactPlayerEvent
  (bind _returnvalue (Transformation|GetActorLocation))
  (bind (_x _y _z) (Math|Vector|BreakVector _returnvalue))
  ;[1 1 1] Impact feedback
  (Effects|SpawnEmitteratLocation (Variables|Default|GetimpactParticle_ref) (Math|Vector|MakeVector (+ _x 5e+01) _y (+ _z 2e+01)))
  ;[1 1 1] Vibration feedback
  (Game|Feedback|PlayDynamicForceFeedback (Game|GetPlayerController 0) 0.5 0.2 true true true true))

(event Collision|EventActorBeginOverlap
  (params (OtherActor :type Actor%20Object%20Reference)))

(fn ConstructionScript)