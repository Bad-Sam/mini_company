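; Ranged enemy soldier Blueprint that plays impact feedback when its ranged impact event fires.
; The event compares the player's formation with the leader's in a rock-paper-scissors scheme: Triangle against Circle, Line against Triangle, Circle against Line.
; Those matchups spawn an enlarged impact particle with stronger controller vibration; others get normal feedback.
; The construction script caches the player reference used by this check.
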(event Custom|ImpactRangedEvent
  (bind _returnvalue (Transformation|GetActorLocation))
  (bind _returnvalue_2 (Transformation|GetActorLocation))
  (bind _playerclass_ref (Variables|Default|GetplayerClass_ref))
  (bind _leader (Variables|Default|GetLeader))
  (bind (_x _y _z) (Math|Vector|BreakVector _returnvalue))
  (bind (_x_2 _y_2 _z_2) (Math|Vector|BreakVector _returnvalue_2))
  (bind _formation (Variables|/Script/MiniCompany.CompanyLeader|GetFormation _leader))
  ;[1 1 1] Impact feedback
  ;;[1 1 1] Determine feedback type
  (Utilities|IsValid _playerclass_ref
    (:Is%20Valid
      (switch Utilities|FlowControl|Switch|SwitchonFormationType (Variables|/Script/MiniCompany.CompanyLeader|GetFormation _playerclass_ref)
        (:TRIANGLE
          (if (Utilities|Enum|Equal(Enum) _formation "CIRCLE")
            ;;[1 1 1] Big feedback
            (Effects|SpawnEmitteratLocation (Variables|Default|GetimpactParticle_ref) (Math|Vector|MakeVector (+ _x_2 5e+01) _y_2 (+ _z_2 2e+01)) (Transformation|GetActorRotation) "2.000000,2.000000,2.000000" :!label _label)
            ;[1 1 1] Vibration feedback
            (Game|Feedback|PlayDynamicForceFeedback (Game|GetPlayerController 0) 0.7 0.2 true true true true)
            (else
              ;;[1 1 1] Nomal feedback
              (Effects|SpawnEmitteratLocation (Variables|Default|GetimpactParticle_ref) (Math|Vector|MakeVector (+ _x 5e+01) _y (+ _z 2e+01)) (Transformation|GetActorRotation) :!label _label_2)
              (Game|Feedback|PlayDynamicForceFeedback (Game|GetPlayerController 0) 0.4 0.2 true true true true))))
        (:LINE
          (if (Utilities|Enum|Equal(Enum) _formation "TRIANGLE")
            (goto _label)
            (else
              (goto _label_2))))
        (:CIRCLE
          (if (Utilities|Enum|Equal(Enum) _formation "LINE")
            (goto _label)
            (else
              (goto _label_2))))))))

(event Collision|EventActorBeginOverlap
  (params (OtherActor :type Actor%20Object%20Reference)))

(event EventTick
  (params (DeltaSeconds :type Float%20%28single-precision%29))
  (|CallParentFunction DeltaSeconds) ; This node is disabled and will not be called.\nDrag off pins to build functionality.
)

(fn ConstructionScript
  (|CallParentFunction)
  (Variables|Default|SetPlayerClass_ref (Utilities|ResolveSoftReference (Variables|Default|Getplayer_ref))))