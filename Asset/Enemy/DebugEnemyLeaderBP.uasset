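; Enemy company leader Blueprint that drives armor and attack feedback and notifies the player pawn when its company is defeated.
; Tick reads armor, health and attack-preparation state to toggle the shield and attack indicators.
; DoOnce gates limit shield changes to one show and one hide, the latter playing an armor-destroyed sound scaled by the game instance's effect volume.
; OnCompanyDeath calls EnemyCompanyDefeated on PlayerBP.
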(event EventOnCompanyDeath
  ;[1 1 1] Sound
  (Default|EnemyCompanyDefeated (.AsPlayer%20BP (Utilities|Casting|CastToPlayerBP (Game|Player|GetPlayerPawn 0)))))

(event EventBeginPlay
  ;[1 1 1] Armor feedback
  ;;[1 1 1] Set feedback visible or not
  (if (> (Variables|Default|GetMaxArmorValue) 0)
    (Rendering|SetVisibility (Variables|Default|GetShieldFeedback) true false)))

(event EventTick
  (params (DeltaSeconds :type Float%20%28single-precision%29))
  (bind _shieldfeedback (Variables|Default|GetShieldFeedback))
  ;[1 1 1] Armor feedback
  ;;[1 1 1] Updating feedback
  (Utilities|FlowControl|Sequence
    (:then_0
      (if (<= (Variables|Default|GetArmorValue) 0)
        (Utilities|FlowControl|DoOnce false
          (:Completed
            (Rendering|SetVisibility _shieldfeedback false false)
            ;[1 1 1] Sound
            (Audio|PlaySoundatLocation "/Game/Asset/Sounds/Armure_détruite/armor_destroyed.armor_destroyed" (Transformation|GetActorLocation) "0, 0, 0" (* (Variables|/Script/MiniCompany.MyGameInstanceMiniCompany|GetEffectVolume (.AsMy%20Game%20Instance%20Mini%20Company (Utilities|Casting|CastToMyGameInstanceMiniCompany (Game|GetGameInstance)))) 0.75) 1.0 0.0 "/Game/Asset/Sounds/SoundAttenuation.SoundAttenuation" 0 0)))
        (else
          (Utilities|FlowControl|DoOnce false
            (:Completed
              (Rendering|SetVisibility _shieldfeedback true false))))))
    (:then_1
      ;[1 1 1] Attack feedback
      (if (> (Variables|Default|GetHealth) 0.0)
        (if (Variables|Default|GetPreparingAttack)
          (Rendering|SetVisibility (Variables|Default|GetAttackFeedback) true false)
          (else
            (Rendering|SetVisibility (Variables|Default|GetAttackFeedback) false false)))))
    (:then_2
      (if (<= (Variables|Default|GetHealth) 0.0)
        (Rendering|SetVisibility (Variables|Default|GetAttackFeedback) false false)))))

(fn ConstructionScript)